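; Demo actor that runs MediaPipe body pose tracking on a playing video and visualizes the result.
; Each tick after Init, it matches the camera aspect ratio to the media and draws the video material into a downscaled render target fed to the tracker.
; While video plays, it optionally draws a debug skeleton colored by landmark visibility and updates the webcam selector UI's color-coded skeleton health bar.
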(event Custom|Shutdown
  (if (Variables|Default|GetbInitialized)
    (Class|MediaPipePoseTrackerComponent|ShutdownGraph (Variables|Default|GetMediaPipePoseTracker))
    (Variables|Default|SetbInitialized false)))

(event Custom|Init
  (Class|MediaPipePoseTrackerComponent|InitGraph (Variables|Default|GetMediaPipePoseTracker))
  (Variables|Default|SetbInitialized true))

(event EventBeginPlay
  (Class|MediaPipePoseTrackerComponent|SetHFoV (Variables|Default|GetMediaPipePoseTracker) (Variables|/Script/Engine.CameraComponent|GetFieldOfView (Variables|/Script/Engine.CameraActor|GetCameraComponent (Variables|Default|GetCamera)))))

(event EventEndPlay
  (params (EndPlayReason :type EEndPlayReason%20Enum :default "Destroyed"))
  (CallFunction|Shutdown))

(event EventTick
  (params (DeltaSeconds :type Float%20%28single-precision%29))
  (bind _mediapipeposetracker (Variables|Default|GetMediaPipePoseTracker))
  (bind _returnvalue (Class|MediaPipePoseTrackerComponent|GetSkeletonHealth _mediapipeposetracker))
  (if (Variables|Default|GetbInitialized)
    (Utilities|FlowControl|Sequence
      (:then_0
        (CallFunction|SetCameraAspectRatio))
      (:then_1
        (CallFunction|RenderTagetResize)
        (if (Audio|Components|Audio|IsPlaying (Variables|Default|GetMediaPlayer))
          (if (Utilities|Enum|Equal(Enum) (Variables|Default|GetVisualizationMode) "Skeleton")
            (CallFunction|DrawDebugSkeleton))
          ;[1 1 1] Skeleton health bar
          (bind _foundwidgets (Widget|GetAllWidgetsOfClass "/Game/WebcamController/UI/W_WebCamSelectorUI.W_WebCamSelectorUI_C" true))
          (Progress|SetPercent (Variables|/Game/WebcamController/UI/W_WebCamSelectorUI.W_WebCamSelectorUI_C|GetPB_SkeletonHealth (Utilities|Array|Get(acopy) _foundwidgets)) _returnvalue)
          (Class|ProgressBar|SetFillColorandOpacity (Variables|/Game/WebcamController/UI/W_WebCamSelectorUI.W_WebCamSelectorUI_C|GetPB_SkeletonHealth (Utilities|Array|Get(acopy) _foundwidgets)) (CallFunction|ColorbyValue _returnvalue))
          (Widget|SetVisibility (Variables|/Game/WebcamController/UI/W_WebCamSelectorUI.W_WebCamSelectorUI_C|GetPB_SkeletonHealth (Utilities|Array|Get(acopy) _foundwidgets)) "Visible")
          (else
            ;[1 1 1] Hide bar if no video playing
            (bind _foundwidgets_2 (Widget|GetAllWidgetsOfClass "/Game/WebcamController/UI/W_WebCamSelectorUI.W_WebCamSelectorUI_C" true))
            (Widget|SetVisibility (Variables|/Game/WebcamController/UI/W_WebCamSelectorUI.W_WebCamSelectorUI_C|GetPB_SkeletonHealth (Utilities|Array|Get(acopy) _foundwidgets_2)) "Hidden")))))))

(fn ConstructionScript)

(fn SetCameraAspectRatio
  ;[1 1 1] Set Camera Aspect Ratio
  (if (Audio|Components|Audio|IsPlaying (Variables|Default|GetMediaPlayer))
    (Class|CameraComponent|SetAspectRatio (Variables|/Script/Engine.CameraActor|GetCameraComponent (Variables|Default|GetCamera)) (Class|MediaTexture|GetAspectRatio (Variables|Default|GetMediaTexture)))
    (else
      (Development|PrintString "SetCameraAspectRatio Waiting..."))))

(fn RenderTagetResize
  ;[1 1 1] Render target - Resizes the input video to 720p -> faster processing
  (Utilities|IsValid (Variables|Default|GetRenderTargetTexture)
    (:Is%20Valid
      (Rendering|DrawMaterialtoRenderTarget (Variables|Default|GetRenderTargetTexture) (Variables|Default|GetVideoMaterial))
      (Class|MediaPipePoseTrackerComponent|GetPoseLandmarksfromRenderTarget2D (Variables|Default|GetMediaPipePoseTracker) (Variables|Default|GetRenderTargetTexture)))))

(fn DrawDebugSkeleton
  (Utilities|FlowControl|Sequence
    (:then_0
      ;[1 1 1] Torso
      (CallFunction|DrawDebugBone 12 11)
      (CallFunction|DrawDebugBone 11 23)
      (CallFunction|DrawDebugBone 23 24)
      (CallFunction|DrawDebugBone 24 12))
    (:then_1
      ;[1 1 1] Left leg
      (CallFunction|DrawDebugBone 24 26)
      (CallFunction|DrawDebugBone 26 28)
      (CallFunction|DrawDebugBone 28 32)
      (CallFunction|DrawDebugBone 32 30)
      (CallFunction|DrawDebugBone 30 28))
    (:then_2
      ;[1 1 1] Right leg
      (CallFunction|DrawDebugBone 23 25)
      (CallFunction|DrawDebugBone 25 27)
      (CallFunction|DrawDebugBone 27 29)
      (CallFunction|DrawDebugBone 29 31)
      (CallFunction|DrawDebugBone 31 27))
    (:then_3
      ;[1 1 1] Left hand
      (CallFunction|DrawDebugBone 12 14)
      (CallFunction|DrawDebugBone 14 16)
      (CallFunction|DrawDebugBone 16 20)
      (CallFunction|DrawDebugBone 20 18)
      (CallFunction|DrawDebugBone 18 16)
      (CallFunction|DrawDebugBone 16 22))
    (:then_4
      ;[1 1 1] Right hand
      (CallFunction|DrawDebugBone 11 13)
      (CallFunction|DrawDebugBone 13 15)
      (CallFunction|DrawDebugBone 15 17)
      (CallFunction|DrawDebugBone 17 19)
      (CallFunction|DrawDebugBone 19 15)
      (CallFunction|DrawDebugBone 15 21))
    (:then_5
      ;[1 1 1] Head
      (CallFunction|DrawDebugBone 10 9)
      (CallFunction|DrawDebugBone 8 6)
      (CallFunction|DrawDebugBone 6 5)
      (CallFunction|DrawDebugBone 5 4)
      (CallFunction|DrawDebugBone 4)
      (CallFunction|DrawDebugBone 0 1)
      (CallFunction|DrawDebugBone 1 2)
      (CallFunction|DrawDebugBone 2 3)
      (CallFunction|DrawDebugBone 3 7))
    (:then_6
      ;[1 1 1] Joints
      (for _index (range 0 32)
        (Class|MediaPipePoseTrackerComponent|DrawPoint (Variables|Default|GetMediaPipePoseTracker) (Class|MediaPipePoseTrackerComponent|GetLandmarkPosition (Variables|Default|GetMediaPipePoseTracker) _index false) "(R=0.000000,G=0.097587,B=0.991102,A=1.000000)" 1e+01 100 0.0)))))

(fn ColorbyValue
  (params (Value :type Float%20%28double-precision%29))
  (if (< Value 0.5)
    (return "(R=1.000000,G=0.000000,B=0.000000,A=1.000000)")
    (elif (>= Value 0.75)
      (return "(R=0.000000,G=1.000000,B=0.000000,A=1.000000)")
      (else
        (return "(R=1.000000,G=0.201022,B=0.000000,A=1.000000)")))))

(fn DrawDebugBone
  (params (Landmark%20ID%20start :type Integer) (Landmark%20ID%20end :type Integer))
  (bind _mediapipeposetracker (Variables|Default|GetMediaPipePoseTracker))
  (Class|MediaPipePoseTrackerComponent|DrawLine (Variables|Default|GetMediaPipePoseTracker) (Class|MediaPipePoseTrackerComponent|GetLandmarkPosition _mediapipeposetracker Landmark%20ID%20start false) (Class|MediaPipePoseTrackerComponent|GetLandmarkPosition _mediapipeposetracker Landmark%20ID%20end false) (CallFunction|ColorbyValue (Class|MediaPipePoseTrackerComponent|GetLandmarkVisibility _mediapipeposetracker Landmark%20ID%20end)) 10 1.0 0.0))