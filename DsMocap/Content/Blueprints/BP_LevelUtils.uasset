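; BP_LevelUtils is a set of level utility functions for preparing a scene that uses a given camera actor, and for quitting the game.
; PreSetup runs three helpers in sequence: cap the frame rate by console command, hide the first DefaultPawn, then set up view and input.
; The last helper switches the first player's view to the passed camera and enables Game and UI input with a visible cursor.
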(fn LimitMaxFpsto120
  ;[1 1 1] Limit max FPS to 120
  (Development|ExecuteConsoleCommand 0 "t.maxfps 120" (Game|GetPlayerController 0)))

(fn HideDefaultPawn
  ;[1 1 1] Hide default pawn
  (bind _outactors (Actor|GetAllActorsOfClass 0 "/Script/Engine.DefaultPawn"))
  (Rendering|SetActorHiddenInGame (Utilities|Array|Get(acopy) _outactors) true))

(fn SetInputModeandCamera
  (params (CameraActor :type Actor%20Object%20Reference))
  (bind _returnvalue (Game|GetPlayerController 0))
  ;[1 1 1] Set input mode, camera
  (Game|Player|SetViewTargetwithBlend (Game|GetPlayerController 0) CameraActor 0.0 "VTBlend_EaseIn" 0.0 false)
  (Input|SetInputModeGameandUI _returnvalue 0 "DoNotLock" false false)
  (Variables|/Script/Engine.PlayerController|SetbShowMouseCursor _returnvalue true))

(fn PreSetup
  (params (CameraActor :type Actor%20Object%20Reference))
  (Utilities|FlowControl|Sequence
    (:then_0
      (CallFunction|LimitMaxFpsto120))
    (:then_1
      (CallFunction|HideDefaultPawn))
    (:then_2
      (CallFunction|SetInputModeandCamera CameraActor))))

(fn QuitPlayerGame
  (Game|QuitGame 0 (Game|GetPlayerController 0) "Quit" true))